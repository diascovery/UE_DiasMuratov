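; Zombie enemy character that punches the player and explodes with a sound on death.
; Tick updates a camera-facing health bar from HealthComponent and rebinds the anim Blueprint's punch event each frame.
; That event enables PunchSphere overlaps, which damage the player once, then switch off.
; Incoming damage feeds HealthComponent, whose OnDeath destroys the actor; custom events start the attack montage and yaw it toward the player.
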(event `CustomEvent`
  (params (DeltaSeconds :type "Float (single-precision)"))
  (`self.RotateTowardsPlayer`))

(event `self.ReceiveTick`
  (params (DeltaSeconds :type "Float (single-precision)"))
  (bind _health_bar_widget (`self.Health Bar Widget`))
  (bind _aswb_health_bar_enemy (cast `/Game/Enemy/WB_HealthBarEnemy` (`WidgetComponent.GetWidget` (`self.Health Bar Widget`))))
  (`ProgressBar.SetPercent` (`/Game/Enemy/WB_HealthBarEnemy.HealthBarEnemy` _aswb_health_bar_enemy) (/ (`/Game/Health/HealthComponent.Health` (`self.HealthComponent`)) 100.0))
  (`SceneComponent.K2_SetWorldRotation` _health_bar_widget (`KismetMathLibrary.FindLookAtRotation` (`SceneComponent.K2_GetComponentLocation` _health_bar_widget) (`SceneComponent.K2_GetComponentLocation` (`PlayerCameraManager.TransformComponent` (`GameplayStatics.GetPlayerCameraManager` 0)))) false false)
  (bind _asabp_zombie (cast `/Game/Characters/Zombie/ABP_Zombie` (`SkeletalMeshComponent.GetAnimInstance` (`self.Mesh`))))
  (add `/Game/Characters/Zombie/ABP_Zombie.OnAttackPunch` _asabp_zombie (delegate `OnAttackPunch`)))

(event `OnAttackPunch`
  (set `PrimitiveComponent.bGenerateOverlapEvents` true (`self.PunchSphere`)))

(event `self.ReceiveAnyDamage`
  (params (Damage :type "Float (single-precision)") (DamageType :type "DamageType Object Reference") (InstigatedBy :type "Controller Object Reference") (DamageCauser :type "Actor Object Reference"))
  (`/Game/Health/HealthComponent.SetDamage` (`self.HealthComponent`) Damage))

(event `RotateTowardsPlayer`
  (bind (_returnvalue_roll _returnvalue_pitch) (`KismetMathLibrary.BreakRotator` (`self.K2_GetActorRotation`)))
  (bind (_returnvalue_roll_2 _returnvalue_pitch_2 _returnvalue_yaw) (`KismetMathLibrary.BreakRotator` (`KismetMathLibrary.FindLookAtRotation` (`self.K2_GetActorLocation`) (`self.K2_GetActorLocation` (`GameplayStatics.GetPlayerCharacter` 0)))))
  (`self.K2_SetActorRotation` (`KismetMathLibrary.MakeRotator` _returnvalue_roll _returnvalue_pitch _returnvalue_yaw)))

(event `self.HealthComponent.OnDeath`
  (`Controller.UnPossess` (`self.GetController`))
  (`self.K2_DestroyActor`)
  (`GameplayStatics.SpawnEmitterAtLocation` "/Game/StarterContent/Particles/P_Explosion.P_Explosion" (`self.K2_GetActorLocation`))
  (`GameplayStatics.PlaySoundAtLocation` "/Game/Audio/Cue/ZombieDeathCue.ZombieDeathCue" (`self.K2_GetActorLocation`) (struct) 1.0 1.0 0.0 null null null null))

(event `self.PunchSphere.OnComponentBeginOverlap`
  (params (OverlappedComponent :type "PrimitiveComponent Object Reference") (OtherActor :type "Actor Object Reference") (OtherComp :type "PrimitiveComponent Object Reference") (OtherBodyIndex :type Integer) (bFromSweep :type Boolean) (SweepResult :type "HitResult Structure (by ref)"))
  (bind _asbp_third_person_character (cast `/Game/ThirdPerson/Blueprints/BP_ThirdPersonCharacter` OtherActor))
  (`GameplayStatics.ApplyDamage` _asbp_third_person_character 20.0 (`self.GetController`) self)
  (set `PrimitiveComponent.bGenerateOverlapEvents` false (`self.PunchSphere`)))

(event `StartAttackAnimation`
  (`|PlayMontage` (`self.Mesh`) "/Game/Characters/Zombie/Animations/Zombie_Attack_Montage.Zombie_Attack_Montage"))

(fn `UserConstructionScript`)