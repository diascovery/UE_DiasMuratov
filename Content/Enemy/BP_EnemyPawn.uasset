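; BP_EnemyPawn is an enemy pawn that constantly turns to face the player and can be destroyed by damage.
; Each Tick sets its yaw toward the player character, leaving pitch and roll unchanged.
; Incoming damage passes to a HealthComponent, whose OnDeath event unpossesses the controller, destroys the actor and spawns an explosion emitter at its location.
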(event `self.ReceiveAnyDamage`
  (params (Damage :type "Float (single-precision)") (DamageType :type "DamageType Object Reference") (InstigatedBy :type "Controller Object Reference") (DamageCauser :type "Actor Object Reference"))
  (`/Game/Health/HealthComponent.SetDamage` (`self.HealthComponent`) Damage))

(event `self.HealthComponent.OnDeath`
  (`Controller.UnPossess` (`self.GetController`))
  (`self.K2_DestroyActor`)
  (`GameplayStatics.SpawnEmitterAtLocation` "/Game/StarterContent/Particles/P_Explosion.P_Explosion" (`self.K2_GetActorLocation`)))

(event `RotateTowardsPlayer`
  (bind (_returnvalue_roll _returnvalue_pitch) (`KismetMathLibrary.BreakRotator` (`self.K2_GetActorRotation`)))
  (bind (_returnvalue_roll_2 _returnvalue_pitch_2 _returnvalue_yaw) (`KismetMathLibrary.BreakRotator` (`KismetMathLibrary.FindLookAtRotation` (`self.K2_GetActorLocation`) (`self.K2_GetActorLocation` (`GameplayStatics.GetPlayerCharacter` 0)))))
  (`self.K2_SetActorRotation` (`KismetMathLibrary.MakeRotator` _returnvalue_roll _returnvalue_pitch _returnvalue_yaw)))

(event `self.ReceiveTick`
  (params (DeltaSeconds :type "Float (single-precision)"))
  (`self.RotateTowardsPlayer`))

(fn `UserConstructionScript`)