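; Game mode for SurviveIO, a survival match the player wins by lasting until a one-second looping countdown reaches zero, which pauses the game.
; On BeginPlay it starts every BP_Spawner and hooks each spawned enemy's HealthComponent death to add score on GS_SurviveIO.
; The SpawnDefaultPawnAtTransform override binds a death event on NewPlayer's HealthComponent.
; Player death prints Game Over and ends all spawners, without clearing the countdown.
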(event `self.ReceiveBeginPlay`
  (bind _returnvalue (`KismetSystemLibrary.K2_SetTimerDelegate` (delegate `CountdownUpdate`) 1.0 true))
  (bind _outactors (`GameplayStatics.GetAllActorsOfClass` "/Game/Enemy/BP_Spawner.BP_Spawner_C"))
  (for _array_element _outactors
    (`/Game/Enemy/BP_Spawner.OnGameStart` _array_element)
    (add `/Game/Enemy/BP_Spawner.OnEnemySpawn` _array_element (delegate `OnEnemySpawn`))))

(event `CountdownUpdate`
  (bind _output_get (set `self.TimeRemaining` (- (`self.TimeRemaining`) 1.0)))
  (`KismetSystemLibrary.PrintString` (`KismetStringLibrary.BuildString_Double` "" "Time Left To Win:" (`self.TimeRemaining`)) true true (struct :`G` 0.13174 :`B` 1.0 :`A` 1.0) 1.0)
  (if (<= _output_get 0.0)
    (`KismetSystemLibrary.K2_ClearAndInvalidateTimerHandle` (stale `self.ReceiveBeginPlay` _returnvalue))
    (`self.GameWon`)))

(event `OnEnemySpawn`
  (params (SpawnedActor :type "Actor Object Reference"))
  (add `/Game/Health/HealthComponent.OnDeath` (`self.GetComponentByClass` SpawnedActor "/Game/Health/HealthComponent.HealthComponent_C") (delegate `OnEnemyDeath`)))

(event `OnEnemyDeath`
  (bind _asgs_survive_io (cast `/Game/SurviveIO/GS_SurviveIO` (`GameplayStatics.GetGameState`)))
  (`/Game/SurviveIO/GS_SurviveIO.AddScore` _asgs_survive_io 20.0))

(event `GameWon`
  (`self.DisableInput` null)
  (`KismetSystemLibrary.PrintString` "YOU WON!" true true (struct :`G` 0.66 :`B` 1.0 :`A` 1.0) 10.0)
  (`GameplayStatics.SetGamePaused` true))

(event `OnPlayerDeath`
  (`self.OnGameOver`))

(event `OnGameOver`
  (`KismetSystemLibrary.PrintString` "Game Over" true true (struct :`R` 1.0 :`A` 1.0) 15.0)
  (bind _outactors (`GameplayStatics.GetAllActorsOfClass` "/Game/Enemy/BP_Spawner.BP_Spawner_C"))
  (for _array_element _outactors
    (`/Game/Enemy/BP_Spawner.OnGameEnd` _array_element)))

(fn `SpawnDefaultPawnAtTransform`
  (params (NewPlayer :type "Controller Object Reference") (SpawnTransform :type "Transform Structure (by ref)"))
  (returns (ReturnValue :type "Pawn Object Reference"))
  (bind _returnvalue (`parent.SpawnDefaultPawnAtTransform` NewPlayer SpawnTransform))
  (add `/Game/Health/HealthComponent.OnDeath` (`self.GetComponentByClass` NewPlayer "/Game/Health/HealthComponent.HealthComponent_C") (`|CreateDelegate` :!event `OnPlayerDeath`))
  (return _returnvalue))

(fn `UserConstructionScript`)